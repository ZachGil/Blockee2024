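; Game mode for BlockHead that runs level flow, from HUD setup to level transitions and the win/lose screen.
; BeginPlay creates the HUD, caches BP_GameInstance and sets game-only input, while Tick prints TotalScore every frame.
; LevelComplete shows a transition widget, then a timer calls LoadNextLevel, which opens the next level or triggers GameComplete on the final one.
; RestartGame resets the game instance and reopens its current level name.
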(event `self.ReceiveBeginPlay`
  ;[0.1062 1 0.2026] Begin Play Sequence
  (`|ExecutionSequence`
    (:`then_0`
      ;[0.1062 1 0.2026] Add HUD to Viewport
      (bind _returnvalue (`|CreateWidget` "/Game/BlockHead/Core/UI/WBP_HUD.WBP_HUD_C"))
      (set `self.HUD` _returnvalue)
      (`UserWidget.AddToViewport` (`self.HUD`) 0))
    (:`then_1`
      ;[0.1062 1 0.2026] Get a Reference to the Game Instance
      (bind _asbp_game_instance (cast `/Game/BlockHead/Core/Game/BP_GameInstance` (`GameplayStatics.GetGameInstance`)))
      (set `self.GameInstance` _asbp_game_instance))
    (:`then_2`
      ;[0.1062 1 0.2026] Hide Mouse Pointer and Set Input Mode to Game Only (Capture Keyboard Input Automatically)
      (`/Game/BlockHead/Core/Game/BP_GameInstance.InputModeGame` (`self.GameInstance`)))))

(event `self.ReceiveTick`
  (params (DeltaSeconds :type "Float (single-precision)"))
  (`KismetSystemLibrary.PrintString` (`KismetStringLibrary.Conv_Int64ToString` (`self.TotalScore`))))

(fn `GameComplete`
  (params (PlayerWon :type Boolean))
  (locals (GameCompleteWidget :type "/Game/BlockHead/Core/UI/WBP_GameComplete Object Reference") (CustomMessage :type Text))
  ;[0.1062 1 0.2026] Set a Custom Message Depending on If Player Has Won or Lost the Game
  (if PlayerWon
    (set `local.CustomMessage` "You Win!")
    (else
      (set `local.CustomMessage` "You Lose!")))
  ;[0.1062 1 0.2026] Show the Game Complete Widget With the Custom Message
  (bind _returnvalue (`|CreateWidget` "/Game/BlockHead/Core/UI/WBP_GameComplete.WBP_GameComplete_C"))
  (set `local.GameCompleteWidget` _returnvalue)
  (set `TextBlock.Text` (`local.CustomMessage`) (`/Game/BlockHead/Core/UI/WBP_GameComplete.LostOrCompleted` (`local.GameCompleteWidget`)))
  (`UserWidget.AddToViewport` (`local.GameCompleteWidget`) 0))

(fn `LevelComplete`
  ;[0.1062 1 0.2026] Show the Level Transition Widget
  (bind _returnvalue (`|CreateWidget` "/Game/BlockHead/Core/UI/WBP_LevelComplete.WBP_LevelComplete_C"))
  (`UserWidget.AddToViewport` _returnvalue 0)
  (`KismetSystemLibrary.K2_SetTimer` null "LoadNextLevel" 2.0))

(fn `LoadNextLevel`
  ;[0.1062 1 0.2026] Load Next Level or Show Game Complete Widget?
  (bind _isfinallevel (`/Game/BlockHead/Core/Game/BP_GameInstance.IsPlayerOnFinalLevel` (`self.GameInstance`)))
  (if _isfinallevel
    ;[0.1062 1 0.2026] Player Has Won the Full Game: Show Game Complete Widget
    (`self.GameComplete` true)
    (else
      ;[0.1062 1 0.2026] Player Has Completed The Level (More Levels To Go): Open Next Level
      (`/Game/BlockHead/Core/Game/BP_GameInstance.NextLevel` (`self.GameInstance`))
      (bind _levelname (`/Game/BlockHead/Core/Game/BP_GameInstance.GetLevelName` (`self.GameInstance`)))
      (`GameplayStatics.OpenLevel` _levelname))))

(fn `RestartGame`
  ;[0.1062 1 0.2026] Restart the Game Via the Game Instance
  (`/Game/BlockHead/Core/Game/BP_GameInstance.ResetInstance` (`self.GameInstance`))
  (bind _levelname (`/Game/BlockHead/Core/Game/BP_GameInstance.GetLevelName` (`self.GameInstance`)))
  (`GameplayStatics.OpenLevel` _levelname))

(fn `UserConstructionScript`)